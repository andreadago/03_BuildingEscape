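; Openable door actor that swings open and closed in response to OpenDoor open and close events.
; On begin play it caches its initial rotation and location.
; A timeline drives a yaw swing combined with the initial rotation, and a timeline event track plays a lock sound at the door's location.
; Closing reverses the same timeline.
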(event OnClose(OpenDoor)
  (bind _doorswing (Timeline|Timeline_0 Reverse)
    (:Update
      (Transformation|SetActorRotation (Math|Rotator|CombineRotators (Math|Rotator|MakeRotator 0.0 0.0 _doorswing) (Variables|Default|GetInitial%20Rotation))))
    (:Play%20Sound
      (Audio|PlaySoundatLocation "/Game/Audio/door-lock.door-lock" (Variables|Default|GetActor%20Location)))))

(event OnOpen(OpenDoor)
  (bind _doorswing (Timeline|Timeline_0 Play)
    (:Update
      (Transformation|SetActorRotation (Math|Rotator|CombineRotators (Math|Rotator|MakeRotator 0.0 0.0 _doorswing) (Variables|Default|GetInitial%20Rotation))))
    (:Play%20Sound
      (Audio|PlaySoundatLocation "/Game/Audio/door-lock.door-lock" (Variables|Default|GetActor%20Location)))))

(event EventBeginPlay
  (Variables|Default|SetInitial%20Rotation (Transformation|GetActorRotation)) ; ActorRotation is "Promoted to variable"
  (Variables|Default|SetActor%20Location (Transformation|GetActorLocation)))

(fn ConstructionScript)